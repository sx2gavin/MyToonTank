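; Toon Tank game mode Blueprint that manages the start, score and game over UI for a match.
; Game events create the start widget with the startup delay, then a score widget that refreshes on each score update.
; On game over it removes the score widget and shows the outcome and final score, binding the restart button to reopen the Prototype level.
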(event `self.GameStartMenu`
  (`self.CreateGameStartWidget`))

(event `self.GameStart`
  (bind _returnvalue (`|CreateWidget` "/Game/Blueprints/UI/WB_Score.WB_Score_C"))
  (bind _output_get (set `self.ScoreWidget` _returnvalue))
  (`/Game/Blueprints/UI/WB_Score.SetScore` _output_get 0)
  (`UserWidget.AddToViewport` _output_get 0))

(event `self.GameOver`
  (params (PlayerHasDied :type Boolean))
  (bind _returnvalue (`|CreateWidget` "/Game/Blueprints/UI/WB_GameOver.WB_GameOver_C"))
  (`/Game/Blueprints/UI/WB_GameOver.SetPlayerHasDied` _returnvalue PlayerHasDied)
  (`/Game/Blueprints/UI/WB_GameOver.SetScore` _returnvalue (`self.PlayerScore`))
  (`UserWidget.AddToPlayerScreen` _returnvalue 0)
  (add `Button.OnClicked` (`/Game/Blueprints/UI/WB_GameOver.RestartButton` _returnvalue) (delegate `RestartLevel`))
  (`Widget.RemoveFromParent` (`self.ScoreWidget`)))

(event `RestartLevel`
  (`GameplayStatics.OpenLevel` "Prototype"))

(event `self.PlayerScoreUpdated`
  (params (Score :type Integer))
  (bind _scorewidget (`self.ScoreWidget`))
  (`/Engine/EditorBlueprintResources/StandardMacros.IsValid` _scorewidget
    (:`Is Valid`
      (`/Game/Blueprints/UI/WB_Score.SetScore` _scorewidget Score))))

(fn `CreateGameStartWidget`
  (bind _returnvalue (`|CreateWidget` "/Game/Blueprints/UI/WB_GameStart.WB_GameStart_C"))
  (`/Game/Blueprints/UI/WB_GameStart.SetDelayTime` _returnvalue (`self.StartUpDelay`))
  (`UserWidget.AddToPlayerScreen` _returnvalue 0))

(fn `UserConstructionScript`)